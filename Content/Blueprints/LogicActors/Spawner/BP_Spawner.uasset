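; BP_Spawner is a logic actor that spawns actors when its linked Button is switched on.
; On BeginPlay, only the authority binds PressDown to the Button's switch-on dispatcher, which calls Spawn.
; Spawn creates one actor of ActorToSpawn's class for each PlacesToSpawn transform.
; Each location is a world-axis offset from the root, while rotation and scale apply as stored, independent of the spawner's own.
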(event Custom|PressDown
  (params (ActivatorId :type Integer))
  (CallFunction|Spawn))

(event Custom|Spawn
  (for _array_element (Variables|Default|GetPlacesToSpawn)
    (Game|SpawnActorfromClass (Utilities|GetClass (Variables|Default|GetActorToSpawn)) (Math|Transform|MakeTransform (+ (Transformation|GetWorldLocation (Variables|Default|GetDefaultSceneRoot)) (.Location (Math|Transform|BreakTransform _array_element))) (.Rotation (Math|Transform|BreakTransform _array_element)) (.Scale (Math|Transform|BreakTransform _array_element))) "Undefined" 0 0)))

(event EventBeginPlay
  (Networking|SwitchHasAuthority
    (:Authority
      (EventDispatchers|BindEventtoSwitchonDispatch (Variables|Default|GetButton) (delegate Custom|PressDown)))))

(fn ConstructionScript)