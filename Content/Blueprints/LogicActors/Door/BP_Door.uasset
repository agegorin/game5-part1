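; BP_Door is a door that swings open once all of its linked activators are on at the same time, and has no logic to close again.
; On BeginPlay the server gives each activator an index, binds its switch on/off dispatchers, and seeds Counter states by comparing current to target value.
; Authority-only handlers update a boolean array, and when all are true a one-shot event plays a rotation timeline on the door.
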(event Custom|OneButtonPressed
  (params (ActivatorId :type Integer))
  (Utilities|FlowControl|Sequence
    (:then_0
      (Networking|SwitchHasAuthority
        (:Authority
          (Utilities|Array|SetArrayElem (Variables|Default|GetActivated) ActivatorId true)
          ;[1 1 1] All Checked?
          (Variables|Default|SetTempActivated true)
          (for _array_element (Variables|Default|GetActivated)
            (Variables|Default|SetTempActivated (and _array_element (Variables|Default|GetTempActivated))))
          (if (Variables|Default|GetTempActivated)
            (CallFunction|OpenDoorEvent)))))
    (:then_1
      (Development|PrintString (Utilities|String|ToString(Integer) ActivatorId)))))

(event Custom|OneButtonUnpressed
  (params (ActivatorId :type Integer))
  (Networking|SwitchHasAuthority
    (:Authority
      (Utilities|Array|SetArrayElem (Variables|Default|GetActivated) ActivatorId false))))

(event Custom|OpenDoorEvent
  (if (not (Variables|Default|GetDoorOpened))
    (Variables|Default|SetDoorOpened true)
    ;[1 1 1] Open Door Animation
    (bind _opendoor (Timeline|OpenDoor Play)
      (:Update
        (Transformation|SetRelativeRotation (Variables|Default|GetDoor) (Math|Rotator|MakeRotator 0.0 0.0 _opendoor) false false)))))

(event EventBeginPlay
  (Networking|SwitchHasAuthority
    (:Authority
      (for (_array_element _array_index) (Variables|Default|GetActivators)
        (Variables|/Game/Blueprints/LogicActors/Door/BP_Activator.BP_Activator_C|Setid _array_element _array_index)
        (EventDispatchers|BindEventtoSwitchOffDispatch _array_element (delegate Custom|OneButtonUnpressed))
        (EventDispatchers|BindEventtoSwitchonDispatch _array_element (delegate Custom|OneButtonPressed))
        (Utilities|Array|Add (Variables|Default|GetActivated) false)
        (bind _asbp_counter (Utilities|Casting|CastToBP_Counter _array_element))
        (Utilities|Array|SetArrayElem (Variables|Default|GetActivated) (Variables|/Game/Blueprints/LogicActors/Door/BP_Activator.BP_Activator_C|Getid _asbp_counter) (== (Variables|/Game/Blueprints/LogicActors/Counter/BP_Counter.BP_Counter_C|GetTargetValue _asbp_counter) (Variables|/Game/Blueprints/LogicActors/Counter/BP_Counter.BP_Counter_C|GetCurrentValue _asbp_counter)))))))

(fn ConstructionScript)

(fn OnRepDoorOpened)