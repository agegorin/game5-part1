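; BP_Counter is a logic actor that acts as a single-digit counter switch, signalling on when its value matches a target.
; On the server, it binds to its Button's switch-on dispatch, and each press advances the value, wrapping from nine to zero.
; At start and after every press, it fires switch-on or switch-off dispatches with its Id.
; The RepNotify on the replicated value updates the displayed number text.
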(event Custom|PressDown
  (params (ActivatorId :type Integer))
  (bind _id (Variables|Default|Getid))
  (Networking|SwitchHasAuthority
    (:Authority
      (Variables|Default|SetCurrentValue (Class|KismetMathLibrary|PercentByteByte (+ (Variables|Default|GetCurrentValue) 1) 10))
      (if (== (Variables|Default|GetCurrentValue) (Variables|Default|GetTargetValue))
        (Default|CallSwitchonDispatch _id)
        (else
          (Default|CallSwitchOffDispatch _id))))))

(event EventBeginPlay
  (bind _id (Variables|Default|Getid))
  (Networking|SwitchHasAuthority
    (:Authority
      (EventDispatchers|BindEventtoSwitchonDispatch (Variables|Default|GetButton) (delegate Custom|PressDown))
      (Variables|Default|SetCurrentValue 0)
      (if (== (Variables|Default|GetCurrentValue) (Variables|Default|GetTargetValue))
        (Default|CallSwitchonDispatch _id)
        (else
          (Default|CallSwitchOffDispatch _id))))))

(fn ConstructionScript)

(fn OnRepCurrentValue
  (Rendering|Components|TextRender|SetText (Variables|Default|GetTR_Number) (Utilities|Text|ToText(String) (Variables|Default|GetCurrentValue))))