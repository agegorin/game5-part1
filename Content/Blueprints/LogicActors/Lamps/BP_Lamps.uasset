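; BP_Lamps is a logic actor showing one lamp per linked activator and firing its own switch-on dispatch when all are on.
; The construction script spawns replicated lamp meshes, evenly spaced across Width.
; On the server, BeginPlay assigns each activator an index Id and binds its on/off dispatches, which update the Activated array and swap that lamp's material.
; It acts as an AND gate, but never fires a switch-off itself.
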(event Custom|ChangeState
  (params (id :type Integer) (lampOn :type Boolean))
  (bind _lamps (Variables|Default|GetLamps))
  (bind _output (Utilities|Array|Get(acopy) _lamps id))
  (if lampOn
    (Rendering|Material|SetMaterial _output 0 "/Game/Blueprints/LogicActors/Lamps/M_LampOn.M_LampOn")
    (else
      (Rendering|Material|SetMaterial _output 0 "/Game/Blueprints/LogicActors/Lamps/M_LampOff.M_LampOff"))))

(event Custom|OneButtonPressed
  (params (ActivatorId :type Integer))
  (Networking|SwitchHasAuthority
    (:Authority
      (Utilities|Array|SetArrayElem (Variables|Default|GetActivated) ActivatorId true)
      (CallFunction|ChangeState ActivatorId true)
      ;[1 1 1] All Checked?
      (Variables|Default|SetTempActivated true)
      (for _array_element (Variables|Default|GetActivated)
        (Variables|Default|SetTempActivated (and _array_element (Variables|Default|GetTempActivated))))
      (if (Variables|Default|GetTempActivated)
        (Default|CallSwitchonDispatch (Variables|Default|Getid))))))

(event Custom|OneButtonUnpressed
  (params (ActivatorId :type Integer))
  (Networking|SwitchHasAuthority
    (:Authority
      (Utilities|Array|SetArrayElem (Variables|Default|GetActivated) ActivatorId false)
      (CallFunction|ChangeState ActivatorId false))))

(event EventBeginPlay
  (Networking|SwitchHasAuthority
    (:Authority
      (for (_array_element _array_index) (Variables|Default|GetActivators)
        (Variables|/Game/Blueprints/LogicActors/Door/BP_Activator.BP_Activator_C|Setid _array_element _array_index)
        (EventDispatchers|BindEventtoSwitchOffDispatch _array_element (delegate Custom|OneButtonUnpressed))
        (EventDispatchers|BindEventtoSwitchonDispatch _array_element (delegate Custom|OneButtonPressed))
        (Utilities|Array|Add (Variables|Default|GetActivated) false)))))

(fn ConstructionScript
  (bind _activators (Variables|Default|GetActivators))
  (bind _width (Variables|Default|GetWidth))
  (|CallParentFunction)
  (for (_ _array_index) _activators
    (bind _returnvalue (AddComponent|AddStaticMeshComponent false))
    (Transformation|SetWorldScale3D _returnvalue "0.200000,0.200000,0.200000")
    (Transformation|SetRelativeLocation _returnvalue (Math|Vector|MakeVector (+ (/ _width -2.0) (* _array_index (/ _width (Math|Conversions|ToFloat(Integer) (- (Utilities|Array|Length _activators) 1))))) 0.0 0.0) false false)
    (Class|ActorComponent|SetIsReplicated _returnvalue true)
    (Utilities|Array|Add (Variables|Default|GetLamps) _returnvalue)))