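; BP_MultiButton is a logic actor that combines several buttons into one switch, signalling on only while all are pressed.
; On BeginPlay the authority gives each entry in ButtonsList its index as Id, binds its on/off dispatches and tracks its state in Activated.
; Each press rechecks every state and fires this actor's own on or off dispatch; any release fires off, all handled on authority only.
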(event Custom|OneButtonPressed
  (params (ActivatorId :type Integer))
  (Utilities|FlowControl|Sequence
    (:then_0
      (Networking|SwitchHasAuthority
        (:Authority
          (Utilities|Array|SetArrayElem (Variables|Default|GetActivated) ActivatorId true)
          ;[1 1 1] All Checked?
          (Variables|Default|SetTempActivated true)
          (for _array_element (Variables|Default|GetActivated)
            (Variables|Default|SetTempActivated (and _array_element (Variables|Default|GetTempActivated))))
          (if (Variables|Default|GetTempActivated)
            (Default|CallSwitchonDispatch (Variables|Default|Getid))
            (else
              (Default|CallSwitchOffDispatch (Variables|Default|Getid)))))))))

(event Custom|OneButtonUnpressed
  (params (ActivatorId :type Integer))
  (Networking|SwitchHasAuthority
    (:Authority
      (Utilities|Array|SetArrayElem (Variables|Default|GetActivated) ActivatorId false)
      (Default|CallSwitchOffDispatch (Variables|Default|Getid)))))

(event EventBeginPlay
  (Networking|SwitchHasAuthority
    (:Authority
      (for (_array_element _array_index) (Variables|Default|GetButtonsList)
        (Variables|/Game/Blueprints/LogicActors/Door/BP_Activator.BP_Activator_C|Setid _array_element _array_index)
        (EventDispatchers|BindEventtoSwitchOffDispatch _array_element (delegate Custom|OneButtonUnpressed))
        (EventDispatchers|BindEventtoSwitchonDispatch _array_element (delegate Custom|OneButtonPressed))
        (Utilities|Array|Add (Variables|Default|GetActivated) false)))))

(fn ConstructionScript
  (|CallParentFunction))

(fn OpenDoorEvent)