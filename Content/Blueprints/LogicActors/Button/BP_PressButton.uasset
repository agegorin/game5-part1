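; BP_PressButton is a floor-style press button that switches an Id on and off as overlaps enter and leave its trigger.
; An overlap counter lets several occupants share it, so only the first entry and last exit act.
; The Press timeline drives the button's height and dynamic-material emissive glow.
; Only the authority dispatches: switch-on after the press finishes forward, switch-off immediately on the last exit.
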(event OnComponentBeginOverlap(Trigger)
  (params (OverlappedComponent :type Primitive%20Component%20Object%20Reference) (OtherActor :type Actor%20Object%20Reference) (OtherComp :type Primitive%20Component%20Object%20Reference) (OtherBodyIndex :type Integer) (bFromSweep :type Boolean) (SweepResult :type Hit%20Result%20Structure%20%28by%20ref%29))
  ;[1 1 1] Check several players on one button
  (bind _result (Math|Integer|IncrementInt (Variables|Default|Getinteractions))
    (:%20%20
      (if (== _result 1)
        ;[1 1 1] Visual
        (bind (_direction _press _glow) (Timeline|Press Play)
          (:Update
            (Transformation|SetRelativeLocation (Variables|Default|GetButton) (Math|Vector|MakeVector 0.0 0.0 _press) false false)
            (Rendering|Material|SetVectorParameterValue (Variables|Default|GetButton%20Material) "Emissive" (Math|Color|Lerp(LinearColor) :B (Variables|Default|GetColor) :Alpha _glow) :!class /Script/Engine.MaterialInstanceDynamic))
          (:Finished
            ;[1 1 1] When pressed down
            (Networking|SwitchHasAuthority
              (:Authority
                (if (Utilities|Enum|Equal(Enum) _direction "Forward")
                  (Default|CallSwitchonDispatch (Variables|Default|Getid)))))))))))

(event OnComponentEndOverlap(Trigger)
  (params (OverlappedComponent :type Primitive%20Component%20Object%20Reference) (OtherActor :type Actor%20Object%20Reference) (OtherComp :type Primitive%20Component%20Object%20Reference) (OtherBodyIndex :type Integer))
  ;[1 1 1] Check several players on one button
  (bind _result (Math|Integer|DecrementInt (Variables|Default|Getinteractions))
    (:%20%20
      (if (== _result 0)
        (Utilities|FlowControl|Sequence
          (:then_0
            ;[1 1 1] When pressed up
            (Networking|SwitchHasAuthority
              (:Authority
                (Default|CallSwitchOffDispatch (Variables|Default|Getid)))))
          (:then_1
            ;[1 1 1] Visual
            (bind (_direction _press _glow) (Timeline|Press Reverse)
              (:Update
                (Transformation|SetRelativeLocation (Variables|Default|GetButton) (Math|Vector|MakeVector 0.0 0.0 _press) false false)
                (Rendering|Material|SetVectorParameterValue (Variables|Default|GetButton%20Material) "Emissive" (Math|Color|Lerp(LinearColor) :B (Variables|Default|GetColor) :Alpha _glow) :!class /Script/Engine.MaterialInstanceDynamic))
              (:Finished
                ;[1 1 1] When pressed down
                (Networking|SwitchHasAuthority
                  (:Authority
                    (if (Utilities|Enum|Equal(Enum) _direction "Forward")
                      (Default|CallSwitchonDispatch (Variables|Default|Getid)))))))))))))

(fn ConstructionScript
  (bind _returnvalue (Rendering|Material|CreateDynamicMaterialInstance (Variables|Default|GetButton) 0 0 "None" :!class /Script/Engine.PrimitiveComponent))
  (Variables|Default|SetButton%20Material _returnvalue))