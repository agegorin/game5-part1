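; BP_PlatformOneWay is a platform that moves one way to TargetPosition when its Button switches on.
; The button is bound only on authority, and a press plays the MovePlatform timeline, scaling the target's relative location and rotation by its alpha with no reverse path.
; The construction script places a TargetPlatform preview and adds a spline toward the destination; the preview is destroyed on BeginPlay.
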(event Custom|PressDown
  (params (ActivatorId :type Integer))
  (CallFunction|Move true))

(event Custom|Move
  (params (isMoving :type Boolean))
  (bind _targetposition (Variables|Default|GetTargetPosition))
  (bind _platform (Variables|Default|GetPlatform))
  (bind (_location _rotation) (Math|Transform|BreakTransform _targetposition))
  (if isMoving
    (bind _main (Timeline|MovePlatform Play)
      (:Update
        (Transformation|SetRelativeTransform _platform (Math|Transform|MakeTransform (* _location _main) (* _rotation _main) (Variables|/Script/Engine.SceneComponent|GetRelativeScale3D _platform)) false false)))))

(event EventBeginPlay
  (Components|DestroyComponent (Variables|Default|GetTargetPlatform))
  (Networking|SwitchHasAuthority
    (:Authority
      (EventDispatchers|BindEventtoSwitchonDispatch (Variables|Default|GetButton) (delegate Custom|PressDown)))))

(fn ConstructionScript
  (bind _targetposition (Variables|Default|GettargetPosition))
  (bind _platform (Variables|Default|GetPlatform))
  (bind (_location _rotation) (Math|Transform|BreakTransform _targetposition))
  (bind _returnvalue (Transformation|GetWorldLocation _platform))
  (Transformation|SetRelativeLocationAndRotation (Variables|Default|GetTargetPlatform) _location _rotation false false)
  (bind _returnvalue_2 (AddComponent|AddSplineComponent false))
  (Spline|SetSplinePoints _returnvalue_2 (Utilities|Array|MakeArray _returnvalue (+ _returnvalue (Math|Vector|RotateVector (.Location (Math|Transform|BreakTransform (Variables|Default|GettargetPosition))) (Transformation|GetWorldRotation _platform)))) "World" true))